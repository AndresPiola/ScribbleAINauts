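; Player Blueprint that fetches a 3D model by keyword at runtime and spawns it in the world.
; TryToRequest passes non-empty keywords to the HttpConnect component, then a random result's model URL is downloaded through glTFRuntime.
; The loaded asset spawns ahead of the player with generated collision, and physics is enabled on its static mesh.
; Request status and download progress are broadcast through event dispatchers.
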(event `self.ReceiveBeginPlay`)

(event `self.HttpConnect.OnRequestReady`
  (params (bSucess :type Boolean) (Results :type "Array of QueryResults Structure"))
  (`self.OnHttpRequest` bSucess)
  (if bSucess
    (`glTFRuntimeFunctionLibrary.glTFLoadAssetFromUrlWithProgress` :`Url` (`.ModelUrl` (break `QueryResults` (`KismetArrayLibrary.Array_Random` Results))) :`Completed` (delegate `OnRemoteActorLoaded`) :`Progress` (delegate `OnDownloadProgress`))))

(event `OnDownloadProgress`
  (params (LoaderConfig :type "glTFRuntimeConfig Structure (by ref)") (BytesProcessed :type Integer) (TotalBytes :type Integer))
  (`self.OnDownloadRequestProgress` false (`KismetMathLibrary.Conv_IntToDouble` (/ BytesProcessed TotalBytes))))

(event `OnRemoteActorLoaded`
  (params (Asset :type "glTFRuntimeAsset Object Reference"))
  (bind (_returnvalue_location _returnvalue_rotation) (`KismetMathLibrary.BreakTransform` (`self.GetTransform`)))
  (bind _returnvalue (`|SpawnActorFromClass` "/Script/glTFRuntime.glTFRuntimeAssetActor" (`KismetMathLibrary.MakeTransform` (+ _returnvalue_location (* (`KismetMathLibrary.GetForwardVector` _returnvalue_rotation) (`self.SpawnDistance`)))) "Undefined" "MultiplyWithRoot" null Asset (make `glTFRuntimeStaticMeshConfig` :`bBuildSimpleCollision` true :`bBuildComplexCollision` true :`CollisionComplexity` "CTF_UseSimpleAndComplex" :`PivotPosition` "Center") (struct) (struct) (struct) true false true true false false false -1 null))
  (bind _returnvalue_2 (`self.GetComponentByClass` _returnvalue "/Script/Engine.StaticMeshComponent"))
  (`/Engine/EditorBlueprintResources/StandardMacros.IsValid` _returnvalue_2
    (:`Is Valid`
      (`PrimitiveComponent.SetSimulatePhysics` _returnvalue_2 true)
      (`self.OnDownloadRequestProgress` true 1.0))))

(fn `TryToRequest`
  (params (Keyword :type String))
  (if (not (`KismetStringLibrary.IsEmpty` Keyword))
    (`HttpConnectComponent.MakeRequest` (`self.HttpConnect`) Keyword)))

(fn `UserConstructionScript`)